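; AI controller for guard NPCs that runs the GuardBehavior behavior tree on the PatrolData blackboard.
; AI perception writes sensed actors lacking the "Enemy" tag to the blackboard's enemy key and clears it when sensing of such an actor fails.
; Each tick it sets the controlled Ue4ASP_Character's Aiming flag according to whether the controller has a valid focus actor.
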(event `self.ReceiveTick`
  (params (DeltaSeconds :type "Float (single-precision)"))
  (bind _asue_4asp_character (cast `/Game/Dynamic/NPC/Behaviour/Ue4ASP_Character` (`self.K2_GetPawn`)))
  (set `/Game/Dynamic/NPC/Behaviour/Ue4ASP_Character.Aiming` (`KismetSystemLibrary.IsValid` (`self.GetFocusActor`)) _asue_4asp_character))

(event `self.ReceiveBeginPlay`
  (bind _blackboardcomponent (`self.UseBlackboard` "/Game/Dynamic/NPC/AI/PatrolData.PatrolData"))
  (`self.RunBehaviorTree` "/Game/Dynamic/NPC/AI/GuardBehavior.GuardBehavior")
  (set `self.Blackboard Component_0` _blackboardcomponent))

(event `self.AIPerception.OnTargetPerceptionUpdated`
  (params (Actor :type "Actor Object Reference") (Stimulus :type "AIStimulus Structure"))
  (bind _enemykey (`self.EnemyKey`))
  (bind _blackboard_component_0 (`self.Blackboard Component_0`))
  (if (`self.ActorHasTag` Actor "Enemy")
    _
    (elif (`.bSuccessfullySensed` (break `AIStimulus` Stimulus))
      (`BlackboardComponent.SetValueAsObject` _blackboard_component_0 _enemykey Actor)
      (else
        (`BlackboardComponent.ClearValue` _blackboard_component_0 _enemykey)))))

(fn `UserConstructionScript`)